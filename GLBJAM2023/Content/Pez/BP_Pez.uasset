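; BP_Pez is a keyboard-controlled fish ("pez") that moves along its local X and Y axes with WASD.
; Key press and release events set one boolean per direction, which Tick checks through a Sequence.
; Each held direction applies a fixed, swept local offset after its own short Delay, without delta-time scaling.
; W and S move along X, A and D along Y.
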(event `Key|A`
  (params (Key :type "Key Structure"))
  ;[0.1906 1 0.2156] Inputs
  (:`Pressed`
    (set `self.A` true))
  (:`Released`
    (set `self.A` false)))

(event `Key|W`
  (params (Key :type "Key Structure"))
  ;[0.1906 1 0.2156] Inputs
  (:`Pressed`
    (set `self.W` true))
  (:`Released`
    (set `self.W` false)))

(event `Key|D`
  (params (Key :type "Key Structure"))
  ;[0.1906 1 0.2156] Inputs
  (:`Pressed`
    (set `self.D` true))
  (:`Released`
    (set `self.D` false)))

(event `Key|S`
  (params (Key :type "Key Structure"))
  ;[0.1906 1 0.2156] Inputs
  (:`Pressed`
    (set `self.S` true))
  (:`Released`
    (set `self.S` false)))

(event `self.ReceiveTick`
  (params (DeltaSeconds :type "Float (single-precision)"))
  ;[1 0.04688 0.04688] Movimiento
  (`|ExecutionSequence`
    (:`then_0`
      (if (`self.A`)
        (`KismetSystemLibrary.Delay` 0.01)
        (`self.K2_AddActorLocalOffset` (0.0 -10.0 0.0) true)))
    (:`then_1`
      (if (`self.D`)
        (`KismetSystemLibrary.Delay` 0.01)
        (`self.K2_AddActorLocalOffset` (0.0 10.0 0.0) true)))
    (:`then_2`
      (if (`self.W`)
        (`KismetSystemLibrary.Delay` 0.01)
        (`self.K2_AddActorLocalOffset` (10.0 0.0 0.0) true)))
    (:`then_3`
      (if (`self.S`)
        (`KismetSystemLibrary.Delay` 0.01)
        (`self.K2_AddActorLocalOffset` (-10.0 0.0 0.0) true)))))

(fn `UserConstructionScript`)