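; BP_CONEJO is a rabbit player pawn whose A, W and D keys change function over time between horizontal movement and jumping.
; BeginPlay resets three direction flipbooks and starts endless 10-second delay loops that set each key's offset and jump flag.
; A and W cycle through left, right and jump out of phase, while D lacks one delay, so only alternates jump and negative movement.
; Tick applies held keys' swept local offsets and jumps.
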(event `Key|A`
  (params (Key :type "Key Structure"))
  ;[0.2214 1 0.008226] Inputs
  (:`Pressed`
    (set `self.A` true))
  (:`Released`
    (set `self.A` false)))

(event `Key|W`
  (params (Key :type "Key Structure"))
  ;[0.2214 1 0.008226] Inputs
  (:`Pressed`
    (set `self.W` true))
  (:`Released`
    (set `self.W` false)))

(event `Key|D`
  (params (Key :type "Key Structure"))
  ;[0.2214 1 0.008226] Inputs
  (:`Pressed`
    (set `self.D` true))
  (:`Released`
    (set `self.D` false)))

(event `self.ReceiveBeginPlay`
  ;[0.7932 0.1229 1] Mecanica
  (`|ExecutionSequence`
    (:`then_0`
      (`PaperFlipbookComponent.SetNewTime` (`self.DerechaFB`) 0.0)
      (`|ExecutionSequence`
        (:`then_0`
          (set `self.Delta Location X A` -10.0 :!label _label)
          (`KismetSystemLibrary.Delay` 10.0)
          (set `self.Delta Location X A` 10.0)
          (`KismetSystemLibrary.Delay` 10.0)
          (set `self.Delta Location X A` 0.0)
          (set `self.AJump` true)
          (`KismetSystemLibrary.Delay` 10.0)
          (set `self.AJump` false)
          (goto _label))
        (:`then_1`
          (set `self.Delta Location X D` 10.0 :!label _label_2)
          (`KismetSystemLibrary.Delay` 10.0)
          (set `self.DJump` true)
          (set `self.Delta Location X D` 0.0)
          (`KismetSystemLibrary.Delay` 10.0)
          (set `self.DJump` false)
          (set `self.Delta Location X D` -10.0)
          (`KismetSystemLibrary.Delay` 10.0)
          (goto _label_2))
        (:`then_2`
          (set `self.WJump` true :!label _label_3)
          (`KismetSystemLibrary.Delay` 10.0)
          (set `self.WJump` false)
          (set `self.Delta Location X W` -10.0)
          (`KismetSystemLibrary.Delay` 10.0)
          (set `self.Delta Location X W` 10.0)
          (`KismetSystemLibrary.Delay` 10.0)
          (set `self.Delta Location X W` 0.0)
          (goto _label_3))))
    (:`then_1`
      (`PaperFlipbookComponent.SetNewTime` (`self.IzquierdaFB`) 0.0))
    (:`then_2`
      (`PaperFlipbookComponent.SetNewTime` (`self.ArribaFB`) 0.0))))

(event `self.ReceiveTick`
  (params (DeltaSeconds :type "Float (single-precision)"))
  ;[1 0 0] Movimiento
  (`|ExecutionSequence`
    (:`then_0`
      (if (`self.A`)
        (`KismetSystemLibrary.Delay` 0.01)
        (`self.K2_AddActorLocalOffset` (`KismetMathLibrary.MakeVector` (`self.Delta Location X A`)) true)
        (if (`self.AJump`)
          (`self.Jump`))))
    (:`then_1`
      (if (`self.D`)
        (`KismetSystemLibrary.Delay` 0.01)
        (`self.K2_AddActorLocalOffset` (`KismetMathLibrary.MakeVector` (`self.Delta Location X D`)) true)
        (if (`self.DJump`)
          (`self.Jump`))))
    (:`then_2`
      (if (`self.W`)
        (`KismetSystemLibrary.Delay` 0.01)
        (`self.K2_AddActorLocalOffset` (`KismetMathLibrary.MakeVector` (`self.Delta Location X W`)) true)
        (if (`self.WJump`)
          (`self.Jump`))))))

(fn `UserConstructionScript`)